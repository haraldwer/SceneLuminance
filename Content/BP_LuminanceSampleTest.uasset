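; BP_LuminanceSampleTest is a test Blueprint that samples scene luminance and shows it through a spotlight's color.
; On BeginPlay it creates a BP_LuminanceTestUI widget, hands itself over as the scene sample, and adds it to the viewport.
; Each tick it queries SceneLuminanceCapture along its eye-view forward vector and applies the result as the referenced Light's spotlight color.
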(event EventBeginPlay
  (bind _returnvalue (UserInterface|CreateWidget "/SceneLuminancePlugin/BP_LuminanceTestUI.BP_LuminanceTestUI_C"))
  (Variables|/SceneLuminancePlugin/BP_LuminanceTestUI.BP_LuminanceTestUI_C|SetSceneSample _returnvalue self)
  (UserInterface|Viewport|AddtoViewport _returnvalue 0))

(event EventTick
  (params (DeltaSeconds :type Float%20%28single-precision%29))
  (Rendering|Components|Light|SetLightColor (Variables|/Script/Engine.SpotLight|GetSpotLightComponent (Variables|Default|GetLight)) (Math|Conversions|ToLinearColor(Color) (Class|SceneLuminanceCaptureComponent|GetLuminance (Variables|Default|GetSceneLuminanceCapture) (Math|Vector|GetForwardVector (.OutRotation (Actor|GetActorEyesViewPoint))))) true))

(fn ConstructionScript)